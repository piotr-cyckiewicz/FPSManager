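; BP_PlayerAvatar is a player entity in a team-based match simulation that can be selected by clicking.
; On BeginPlay it caches the GM_MatchGameplay game mode and the BP_GameSimulationHUD.
; A capsule click is forwarded to the HUD only when the avatar's team matches the game mode's player team.
; CalculatePath returns a synchronous navigation path from the avatar to a given location, using its AI controller as context.
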(event `self.ReceiveBeginPlay`
  (bind _asgm_match_gameplay (cast `/Game/Blueprints/Abstract/GameModes/GM_MatchGameplay` (`GameplayStatics.GetGameMode`)))
  (set `self.GameMode` _asgm_match_gameplay)
  (bind _asbp_game_simulation_hud (cast `/Game/Blueprints/Abstract/GameModes/BP_GameSimulationHUD` (`PlayerController.GetHUD` (`GameplayStatics.GetPlayerController` 0))))
  (set `self.HUD` _asbp_game_simulation_hud))

(event `self.CapsuleComponent.OnClicked`
  (params (TouchedComponent :type "PrimitiveComponent Object Reference") (ButtonPressed :type "Key Structure"))
  ; Player Selection
  (if (== (`self.Team`) (`/Game/Blueprints/Abstract/GameModes/GM_MatchGameplay.GetPlayerTeam` (`self.GameMode`)))
    (`/Game/Blueprints/Abstract/GameModes/BP_GameSimulationHUD.OnPlayerClicked` (`self.HUD`) self)))

(fn `CalculatePath`
  (params (Location :type "Vector Structure"))
  (returns (Path :type "NavigationPath Object Reference"))
  (bind _returnvalue (`NavigationSystemV1.FindPathToLocationSynchronously` (`self.K2_GetActorLocation`) Location (`AIBlueprintHelperLibrary.GetAIController` null) null))
  (return _returnvalue))

(fn `UserConstructionScript`)