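; HUD for the match simulation that tracks the world point under the mouse and shows the options menu for a clicked player.
; On begin play it caches the match controller and camera, creates the player options widget, and records and prints the avatar capsule size.
; Each tick a visibility trace from the camera along the mouse direction updates the stored point.
; Player clicks update the single reused widget, adding it once and closing its task-parameter menu.
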(event `self.ReceiveBeginPlay`
  (`self.InitializeVariables`))

(event `self.ReceiveTick`
  (params (DeltaSeconds :type "Float (single-precision)"))
  (bind (_pointlocation _isvalid) (`self.MouseLineTrace`))
  (if _isvalid
    (set `self.Point Location` _pointlocation)))

(fn `InitializeVariables`
  (bind _aspc_match_gameplay (cast `/Game/Blueprints/Abstract/GameModes/PC_MatchGameplay` (`GameplayStatics.GetPlayerController` 0)))
  (set `self.PlayerController` _aspc_match_gameplay)
  (bind _returnvalue (`|CreateWidget` "/Game/Blueprints/UI/GameSimulation/Widgets/WBP_PlayerOption.WBP_PlayerOption_C"))
  (set `self.PlayerOptionsWidget` _returnvalue)
  (bind _asbp_player_cam (cast `/Game/Blueprints/Entities/BP_PlayerCam` (`GameplayStatics.GetPlayerPawn` 0)))
  (set `self.PlayerCam` (`/Game/Blueprints/Entities/BP_PlayerCam.Camera` _asbp_player_cam))
  (bind _returnvalue_2 (`GameplayStatics.GetActorOfClass` "/Game/Blueprints/Entities/BP_PlayerAvatar.BP_PlayerAvatar_C"))
  (bind (_outradius _outhalfheight) (`CapsuleComponent.GetScaledCapsuleSize` (`Character.CapsuleComponent` _returnvalue_2)))
  (bind _output_get (set `self.AvatarCapsuleSize` (`KismetMathLibrary.MakeVector2D` _outradius _outhalfheight)))
  (`KismetSystemLibrary.PrintString` (`KismetStringLibrary.Conv_Vector2dToString` _output_get)))

(fn `MouseLineTrace`
  (returns (PointLocation :type "Vector Structure") (IsValid :type Boolean) (HitActor :type "Actor Object Reference"))
  (bind _returnvalue (`SceneComponent.K2_GetComponentLocation` (`self.PlayerCam`)))
  (bind (_outhit _returnvalue_2) (`KismetSystemLibrary.LineTraceSingle` _returnvalue (+ _returnvalue (`/Game/Blueprints/Abstract/GameModes/PC_MatchGameplay.GetMouseDirection` (`self.PlayerController`) 100000.0)) "TraceTypeQuery1"))
  (if _returnvalue_2
    (return (`.Location` (`GameplayStatics.BreakHitResult` _outhit)) true (`.HitActor` (`GameplayStatics.BreakHitResult` _outhit)))
    (else
      (return (0.0 0.0 0.0) false null))))

(fn `OnPlayerClicked`
  (params (Player :type "/Game/Blueprints/Entities/BP_PlayerAvatar Object Reference"))
  (bind _playeroptionswidget (`self.PlayerOptionsWidget`))
  ; On Player Clicked
  (`/Game/Blueprints/UI/GameSimulation/Widgets/WBP_PlayerOption.UpdatePlayer` (`self.PlayerOptionsWidget`) Player)
  (if (`self.PlayerOptionsWidgetInViewport`)
    (`/Game/Blueprints/UI/GameSimulation/Widgets/WBP_PlayerOption.CloseParameterTaskMenu` _playeroptionswidget)
    (else
      (`UserWidget.AddToViewport` _playeroptionswidget 0)
      (set `self.PlayerOptionsWidgetInViewport` true)
      (`/Game/Blueprints/UI/GameSimulation/Widgets/WBP_PlayerOption.CloseParameterTaskMenu` _playeroptionswidget))))

(fn `UserConstructionScript`)